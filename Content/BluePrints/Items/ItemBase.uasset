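; Base Blueprint for pickup items, holding an item info struct and a prompt widget for picking the item up.
; On BeginPlay it creates the PickUpText widget from that struct's item and text, then binds PickUpItem to the player IngameCharacter's pickup event.
; PickUpItem only checks range and collision, with no action after the check.
; The range flag is not set here, and the widget is never displayed here.
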(event Custom|PickUpItem
  (if (and (Variables|Default|GetIsInRange) (Collision|GetActorEnableCollision))
    _))

(event EventBeginPlay
  (bind _iteminfo (Variables|Default|GetItemInfo))
  (bind (_item _itemimage _pickuptext) (Utilities|Struct|BreakItemStruct _iteminfo))
  (bind _returnvalue (UserInterface|CreateWidget "/Game/UI/Ingame/PickUpText.PickUpText_C"))
  (Variables|Default|SetPickUpTextWidget _returnvalue)
  (Variables|/Game/UI/Ingame/PickUpText.PickUpText_C|SetPickUpActor _returnvalue _item)
  (Variables|/Game/UI/Ingame/PickUpText.PickUpText_C|SetPickUpText _returnvalue _pickuptext)
  (Utilities|Struct|SetmembersinItemStruct _iteminfo)
  (bind _asingame_character (Utilities|Casting|CastToIngameCharacter (Game|GetPlayerCharacter 0)))
  (Variables|Default|SetIngameCharacter _asingame_character)
  (EventDispatchers|BindEventtoPickUpItem _asingame_character (delegate Custom|PickUpItem)))

(event Collision|EventActorBeginOverlap
  (params (OtherActor :type Actor%20Object%20Reference)))

(event EventTick
  (params (DeltaSeconds :type Float%20%28single-precision%29)))

(fn ConstructionScript)