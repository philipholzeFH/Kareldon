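; Procedural building Blueprint that assembles a multi-storey, grid-based building from modular pieces in its Construction Script, with no runtime logic.
; For each storey from 0 through NumFloor, it adds wall or window instances along four sides, chosen by per-side flags.
; Each side can swap one ground-level segment for a door.
; Floor tile instances fill each level, leaving one configurable stair opening above ground level.
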(event EventBeginPlay)

(event Collision|EventActorBeginOverlap
  (params (OtherActor :type Actor%20Object%20Reference)))

(event EventTick
  (params (DeltaSeconds :type Float%20%28single-precision%29)))

(fn ConstructionScript
  (bind _wallwidth (Variables|Default|GetWallWidth))
  (bind _wallwidth_2 (Variables|Default|GetWallWidth))
  (bind _wallwidth_3 (Variables|Default|GetWallWidth))
  (bind _wallwidth_4 (Variables|Default|GetWallWidth))
  (bind _wallwidth_5 (Variables|Default|GetWallWidth))
  (for _index (range 0 (Variables|Default|GetNumFloor))
    (Variables|Default|SetactualFloorIndex _index)
    ;[0 0.1749 1] Walls
    ;;[1 1 1] Left
    (for _index_2 (range 0 (- (Variables|Default|GetFloorCount_X) 1))
      (if (and (== _index_2 (- (Variables|Default|GetDoor_Left) 1)) (== (Variables|Default|GetactualFloorIndex) 0))
        (Components|InstancedStaticMesh|AddInstance (Variables|Default|GetDoor) (Math|Transform|MakeTransform (Math|Vector|MakeVector (* _index_2 _wallwidth_2) (* 0 _wallwidth_2) (* (Variables|Default|GetactualFloorIndex) _wallwidth_2)) (Math|Rotator|MakeRotator 0.0 0.0 0.0)))
        (elif (Variables|Default|GetWindowLeft)
          (Components|InstancedStaticMesh|AddInstance (Variables|Default|GetWindow) (Math|Transform|MakeTransform (Math|Vector|MakeVector (* _index_2 _wallwidth_2) (* 0 _wallwidth_2) (* (Variables|Default|GetactualFloorIndex) _wallwidth_2)) (Math|Rotator|MakeRotator 0.0 0.0 0.0)))
          (else
            (Components|InstancedStaticMesh|AddInstance (Variables|Default|GetWall) (Math|Transform|MakeTransform (Math|Vector|MakeVector (* _index_2 _wallwidth_2) (* 0 _wallwidth_2) (* (Variables|Default|GetactualFloorIndex) _wallwidth_2)) (Math|Rotator|MakeRotator 0.0 0.0 0.0)))))))
    ;;[1 1 1] right
    (for _index_3 (range 0 (- (Variables|Default|GetFloorCount_X) 1))
      (if (and (== _index_3 (- (Variables|Default|GetDoor_Right) 1)) (== (Variables|Default|GetactualFloorIndex) 0))
        (Components|InstancedStaticMesh|AddInstance (Variables|Default|GetDoor) (Math|Transform|MakeTransform (Math|Vector|MakeVector (* _index_3 _wallwidth_3) (* (Variables|Default|GetFloorCount_Y) _wallwidth_3) (* (Variables|Default|GetactualFloorIndex) _wallwidth_3)) (Math|Rotator|MakeRotator 0.0 0.0 0.0)))
        (elif (Variables|Default|GetWindowRight)
          (Components|InstancedStaticMesh|AddInstance (Variables|Default|GetWindow) (Math|Transform|MakeTransform (Math|Vector|MakeVector (* _index_3 _wallwidth_3) (* (Variables|Default|GetFloorCount_Y) _wallwidth_3) (* (Variables|Default|GetactualFloorIndex) _wallwidth_3)) (Math|Rotator|MakeRotator 0.0 0.0 0.0)))
          (else
            (Components|InstancedStaticMesh|AddInstance (Variables|Default|GetWall) (Math|Transform|MakeTransform (Math|Vector|MakeVector (* _index_3 _wallwidth_3) (* (Variables|Default|GetFloorCount_Y) _wallwidth_3) (* (Variables|Default|GetactualFloorIndex) _wallwidth_3)) (Math|Rotator|MakeRotator 0.0 0.0 0.0)))))))
    ;;[1 1 1] front
    (for _index_4 (range 0 (- (Variables|Default|GetFloorCount_Y) 1))
      (if (and (== _index_4 (- (Variables|Default|GetDoor_Front) 1)) (== (Variables|Default|GetactualFloorIndex) 0))
        (Components|InstancedStaticMesh|AddInstance (Variables|Default|GetDoor) (Math|Transform|MakeTransform (Math|Vector|MakeVector (* 0 _wallwidth_5) (* _index_4 _wallwidth_5) (* (Variables|Default|GetactualFloorIndex) _wallwidth_5)) (Math|Rotator|MakeRotator 0.0 0.0 9e+01)))
        (elif (Variables|Default|GetWindowFront)
          (Components|InstancedStaticMesh|AddInstance (Variables|Default|GetWindow) (Math|Transform|MakeTransform (Math|Vector|MakeVector (* 0 _wallwidth_5) (* _index_4 _wallwidth_5) (* (Variables|Default|GetactualFloorIndex) _wallwidth_5)) (Math|Rotator|MakeRotator 0.0 0.0 9e+01)))
          (else
            (Components|InstancedStaticMesh|AddInstance (Variables|Default|GetWall) (Math|Transform|MakeTransform (Math|Vector|MakeVector (* 0 _wallwidth_5) (* _index_4 _wallwidth_5) (* (Variables|Default|GetactualFloorIndex) _wallwidth_5)) (Math|Rotator|MakeRotator 0.0 0.0 9e+01)))))))
    ;;[1 1 1] back
    (for _index_5 (range 0 (- (Variables|Default|GetFloorCount_Y) 1))
      (if (and (== _index_5 (- (Variables|Default|GetDoor_Back) 1)) (== (Variables|Default|GetactualFloorIndex) 0))
        (Components|InstancedStaticMesh|AddInstance (Variables|Default|GetDoor) (Math|Transform|MakeTransform (Math|Vector|MakeVector (* (Variables|Default|GetFloorCount_X) _wallwidth_4) (* _index_5 _wallwidth_4) (* (Variables|Default|GetactualFloorIndex) _wallwidth_4)) (Math|Rotator|MakeRotator 0.0 0.0 9e+01)))
        (elif (Variables|Default|GetWindowBack)
          (Components|InstancedStaticMesh|AddInstance (Variables|Default|GetWindow) (Math|Transform|MakeTransform (Math|Vector|MakeVector (* (Variables|Default|GetFloorCount_X) _wallwidth_4) (* _index_5 _wallwidth_4) (* (Variables|Default|GetactualFloorIndex) _wallwidth_4)) (Math|Rotator|MakeRotator 0.0 0.0 9e+01)))
          (else
            (Components|InstancedStaticMesh|AddInstance (Variables|Default|GetWall) (Math|Transform|MakeTransform (Math|Vector|MakeVector (* (Variables|Default|GetFloorCount_X) _wallwidth_4) (* _index_5 _wallwidth_4) (* (Variables|Default|GetactualFloorIndex) _wallwidth_4)) (Math|Rotator|MakeRotator 0.0 0.0 9e+01)))))))
    ;[0.4039 0 1] Boden
    (for _index_6 (range 0 (- (Variables|Default|GetFloorCount_Y) 1))
      (for _index_7 (range 0 (- (Variables|Default|GetFloorCount_X) 1))
        (if (not (Math|Boolean|ANDBoolean (== (- (Variables|Default|GetStairs_X) 1) _index_6) (== (- (Variables|Default|GetStairs_Y) 1) _index_7) (!= (Variables|Default|GetactualFloorIndex) 0)))
          (Components|InstancedStaticMesh|AddInstance (Variables|Default|GetFloor) (Math|Transform|MakeTransform (Math|Vector|MakeVector (* _index_7 _wallwidth) (* _index_6 _wallwidth) (* (Variables|Default|GetactualFloorIndex) _wallwidth)))))))))